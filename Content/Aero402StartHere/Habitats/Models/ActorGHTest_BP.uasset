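; Test actor that runs a greenhouse air composition model, tracking O2, CO2 and other gas masses from configured initial values.
; Each tick feeds the stored masses and dummy habitat-to-greenhouse inflow rate and composition into GHAirModelFuncV2, saving the new masses and an emergency leak flag.
; The GHModelSwitch input toggles Hab2GH; when off, Tick zeroes the dummy inflow rate without restoring it.
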(event EventBeginPlay
  (Variables|Default|SetAirMassGH_O2 (Variables|Default|GetAirMass_GH_O2_Initial))
  (Variables|Default|SetAirMassGH_CO2 (Variables|Default|GetAirMass_GH_CO2_Initial))
  (Variables|Default|SetAirMassGH_Other (Variables|Default|GetAirMass_GH_Other_Initial))
  (Input|EnableInput (Game|GetPlayerController 0)))

(event Collision|EventActorBeginOverlap
  (params (OtherActor :type Actor%20Object%20Reference)))

(event EventTick
  (params (DeltaSeconds :type Float%20%28single-precision%29))
  (if (Variables|Default|GetHab2GH)
    _
    (else
      (Variables|Default|SetAirMassRate_Hab2GH_Dummy 0.0)))
  (bind _returnvalue (Class|ActorGHTest|GHAirModelFuncV2 DeltaSeconds (Variables|Default|GetAirMassRate_Hab2GH_Dummy) (Variables|Default|GetAirComp_Hab2GH_O2_Dummy) (Variables|Default|GetAirComp_Hab2GH_CO2_Dummy) (Variables|Default|GetAirComp_Hab2GH_Other_Dummy) (Variables|Default|GetAirMassGH_O2) (Variables|Default|GetAirMassGH_CO2) (Variables|Default|GetAirMassGH_Other)))
  (Variables|Default|SetAirGHNew _returnvalue)
  (Variables|Default|SetAirMassGH_O2 (Utilities|Array|Get(acopy) _returnvalue))
  (Variables|Default|SetAirMassGH_CO2 (Utilities|Array|Get(acopy) _returnvalue 1))
  (Variables|Default|SetAirMassGH_Other (Utilities|Array|Get(acopy) _returnvalue 2))
  (Variables|Default|SetEmergency_LeakGH (> (Utilities|Array|Get(acopy) _returnvalue 7) 0.0)))

(event Input|ActionEvents|InputActionGHModelSwitch
  (params (Key :type Key%20Structure :default "AnyKey"))
  (:Pressed
    (Utilities|FlowControl|FlipFlop
      (:A
        (Variables|Default|SetHab2GH false))
      (:B
        (Variables|Default|SetHab2GH true)))))

(fn ConstructionScript)