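; Moon printer actor that travels along a track spline, simulating a printed path in the ISRU content.
; On BeginPlay a timeline, scaled by Duration and started at an offset, drives location and rotation along the referenced track's spline.
; Each Tick spawns an emitter at the print head and traces down beneath it.
; Nested FlipFlops place a permanent printed-material decal at the trace hit every fourth tick, aligned to head yaw.
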(event Custom|MovePrinter
  (bind _trackref (Variables|Default|GetTrackRef))
  (bind _usefulspline (Variables|/Game/Aero402StartHere/ISRU/Spline/Track.Track_C|GetUsefulSpline _trackref))
  (Components|Timeline|SetPlayRate (Variables|Default|GetPrinterMover) (/ 1.0 (Variables|Default|GetDuration)))
  (Components|Timeline|SetNewTime (Variables|Default|GetPrinterMover) (Variables|Default|GetPrinterStartOffset))
  (bind _newtrack_0 (Timeline|PrinterMover Play)
    (:Update
      (Variables|Default|SetAlpha _newtrack_0)
      (Transformation|SetActorLocationAndRotation (Spline|GetLocationatDistanceAlongSpline _usefulspline (Math|Float|Lerp 0.0 (Spline|GetSplineLength (Variables|/Game/Aero402StartHere/ISRU/Spline/Track.Track_C|GetUsefulSpline (Variables|Default|GetTrackRef))) (Variables|Default|GetAlpha)) "World") (Spline|GetRotationatDistanceAlongSpline _usefulspline (Math|Float|Lerp 0.0 (Spline|GetSplineLength (Variables|/Game/Aero402StartHere/ISRU/Spline/Track.Track_C|GetUsefulSpline (Variables|Default|GetTrackRef))) (Variables|Default|GetAlpha)) "World")))))

(event EventBeginPlay
  (CallFunction|MovePrinter))

(event Collision|EventActorBeginOverlap
  (params (OtherActor :type Actor%20Object%20Reference)))

(event EventTick
  (params (DeltaSeconds :type Float%20%28single-precision%29))
  (bind _printhead (Variables|Default|GetPrintHead))
  (CallFunction|PrintedPath _printhead _printhead)
  (Effects|SpawnEmitteratLocation 0 (Transformation|GetWorldLocation _printhead)))

(fn ConstructionScript)

(fn PrintedPath
  (params (Self2 :type Scene%20Component%20Object%20Reference) (Self3 :type Scene%20Component%20Object%20Reference))
  (bind _returnvalue (Transformation|GetWorldLocation Self2))
  (bind _outhit (Collision|LineTraceByChannel (+ _returnvalue "0, 0,2.000000") (- _returnvalue "0, 0,15.000000") "TraceTypeQuery1" true 0 "None" false))
  (Utilities|FlowControl|FlipFlop
    (:A
      (Utilities|FlowControl|FlipFlop
        (:A
          (Rendering|Decal|SpawnDecalatLocation "/Game/Textures/PrintedMat.PrintedMat" "50.000000,50.000000,50.000000" (.Location (Collision|BreakHitResult _outhit)) (Math|Rotator|MakeRotator 0.0 -9e+01 (- (.yaw (Transformation|GetWorldRotation Self3)) -9e+01)) 0.0))))))