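; Airlock air-mass simulation Blueprint that models pressurization and door-opening air loss, using C++ airlock math functions.
; Each tick with the door closed, it steps the airlock air function with a mass flow rate, scaled by a multiplier in speed mode, and prints the result.
; With the door open, it computes air loss from initial and final moles, calls the open-door function and prints debug text.
; All state flags reset on BeginPlay.
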(event EventBeginPlay
  (Variables|Default|SetbIsOn false)
  (Variables|Default|SetdIsOn false)
  (Variables|Default|SetspeedMode false)
  (Variables|Default|SetdoorOpen false))

(event EventTick
  (params (DeltaSeconds :type Float%20%28single-precision%29))
  (if (Variables|Default|GetdoorOpen)
    (bind _returnvalue (Class|ALAirMathematicalMarkFinal|UALAirMathmaticalMarkGetma0AL))
    (bind _returnvalue_2 (Class|ALAirMathematicalMarkFinal|UALAirMathmaticalMarkGetmafAL))
    (Class|ALAirMathematicalMarkFinal|AirlockLossFunc _returnvalue _returnvalue_2)
    (Class|ALAirMathematicalMarkFinal|UALAirMathmaticalMarkOpenDoor)
    (Development|PrintString "Hello true")
    (elif (Variables|Default|GetspeedMode)
      (bind _returnvalue_3 (Class|ALAirMathematicalMarkFinal|AirlockAirFunc DeltaSeconds (* (Variables|Default|GetspeedMultiplier) (Variables|Default|Getmdot_dumb)) (Variables|Default|GetbIsOn) (Variables|Default|GetdIsOn)))
      (Development|PrintString (Utilities|String|ToString(Float) _returnvalue_3) true true "(R=1.000000,G=0.000000,B=0.038347,A=1.000000)" 0.0)
      (else
        (bind _returnvalue_4 (Class|ALAirMathematicalMarkFinal|AirlockAirFunc DeltaSeconds (Variables|Default|Getmdot_dumb) (Variables|Default|GetbIsOn) (Variables|Default|GetdIsOn)))
        (Development|PrintString (Utilities|String|ToString(Float) _returnvalue_4) true true "(R=1.000000,G=0.000000,B=0.038347,A=1.000000)" 0.0)))))